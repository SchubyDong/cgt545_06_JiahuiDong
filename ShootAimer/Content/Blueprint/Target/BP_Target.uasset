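; BP_Target is a destructible target that plays a sound, spawns a small explosion and destroys itself on its Damage event.
; The construction script gives it a random flattened scale and a random TargetStatus.
; On BeginPlay, that status selects horizontal movement, vertical movement or scale change, all driven by one shared timeline with randomized play rate.
; Movement lerps the Target component toward a random offset, while scaling lerps up from its random size.
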(event `self.ReceiveBeginPlay`
  (bind _returnvalue (`KismetMathLibrary.RandomFloatInRange` 100.0 250.0))
  (bind _random_scale (`self.Random_Scale`))
  (bind _returnvalue_2 (* _random_scale 1.5))
  (switch `/Game/Blueprint/Target/Target_Status` (`self.Target_Status`)
    (:`NewEnumerator1`
      (set `self.Destination` (`KismetMathLibrary.MakeVector` _returnvalue)))
    (:`NewEnumerator2`
      (set `self.Destination` (`KismetMathLibrary.MakeVector` 0.0 0.0 _returnvalue)))
    (:`NewEnumerator3`
      _))
  (`TimelineComponent.SetPlayRate` (`self.Move_Timeline`) (/ 1.0 (`KismetMathLibrary.RandomFloatInRange` 1.5 3.0)))
  (bind (_direction _newtrack_0) (`Timeline|Move_Timeline` :!via `PlayFromStart`)
    (:`Update`
      (switch `/Game/Blueprint/Target/Target_Status` (`self.Target_Status`)
        (:`NewEnumerator1`
          (`SceneComponent.K2_SetRelativeLocation` (`self.Target`) (`KismetMathLibrary.VLerp` (0.0 0.0 0.0) (`self.Destination`) _newtrack_0) false false :!label _label))
        (:`NewEnumerator2`
          (goto _label))
        (:`NewEnumerator3`
          (`SceneComponent.SetRelativeScale3D` (`self.Target`) (`KismetMathLibrary.VLerp` (`KismetMathLibrary.MakeVector` _random_scale _random_scale 0.03) (`KismetMathLibrary.MakeVector` _returnvalue_2 _returnvalue_2 0.03) _newtrack_0)))))))

(event `/Game/Blueprint/Weapons/BPI_Damage.Receive Damage`
  (bind _returnvalue (`SceneComponent.K2_GetComponentLocation` (`self.Target`)))
  (`GameplayStatics.PlaySoundAtLocation` null _returnvalue (struct) 1.0 1.0 0.0 null null null null)
  (`GameplayStatics.SpawnEmitterAtLocation` "/Game/StarterContent/Particles/P_Explosion.P_Explosion" _returnvalue (struct) (0.2 0.2 0.2))
  (`self.K2_DestroyActor`))

(fn `UserConstructionScript`
  (bind _output_get (set `self.Random_Scale` (`KismetMathLibrary.RandomFloatInRange` 0.25 1.0)))
  (`SceneComponent.SetWorldScale3D` (`self.Target`) (`KismetMathLibrary.MakeVector` _output_get _output_get 0.03))
  (set `self.Target_Status` (cast `/Game/Blueprint/Target/Target_Status` (`KismetMathLibrary.Conv_IntToByte` (`KismetMathLibrary.RandomIntegerInRange` 0 3)))))