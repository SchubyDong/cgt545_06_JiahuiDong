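; BP_Target_Spawner spawns BP_Target actors at random points inside a box area whose extent is set in the construction script.
; Spawn_Targets binds SpawnTarget to a looping timer with a zero interval, then calls it in a loop for an initial batch.
; SpawnTarget caps the world's target count, picks a point within half the box extent and rotates each new target toward the player camera.
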(event `Spawn_Targets`
  (`KismetSystemLibrary.K2_SetTimerDelegate` (delegate `SpawnTarget`) 0.0 true)
  (for _ (range 9)
    (`self.SpawnTarget`)))

(event `SpawnTarget`
  (bind _spawn_area (`self.Spawn_Area`))
  (bind _outactors (`GameplayStatics.GetAllActorsOfClass` "/Game/Blueprint/Target/BP_Target.BP_Target_C"))
  (if (<= (`KismetArrayLibrary.Array_Length` _outactors) 11)
    (bind _output_get (set `self.Spawn location` (`KismetMathLibrary.RandomPointInBoundingBox` (`SceneComponent.K2_GetComponentLocation` _spawn_area) (/ (`BoxComponent.BoxExtent` _spawn_area) (2.0 2.0 2.0)))))
    (bind (_returnvalue_roll _returnvalue_pitch _returnvalue_yaw) (`KismetMathLibrary.BreakRotator` (`KismetMathLibrary.FindLookAtRotation` _output_get (`SceneComponent.K2_GetComponentLocation` (`PlayerCameraManager.TransformComponent` (`GameplayStatics.GetPlayerCameraManager` 0))))))
    (`|SpawnActorFromClass` "/Game/Blueprint/Target/BP_Target.BP_Target_C" (`KismetMathLibrary.MakeTransform` _output_get (`KismetMathLibrary.MakeRotator` _returnvalue_roll _returnvalue_pitch _returnvalue_yaw)) "Undefined" "MultiplyWithRoot" null null)))

(fn `UserConstructionScript`
  (`BoxComponent.SetBoxExtent` (`self.Spawn_Area`) (`self. Box_Extent`) true))