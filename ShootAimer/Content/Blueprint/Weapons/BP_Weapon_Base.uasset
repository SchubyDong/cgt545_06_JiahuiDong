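; Base weapon Blueprint that handles ammo, firing and reloading, and doubles as an overlap pickup for the first-person character.
; WeaponFire either triggers a reload or spends ammo, spawns muzzle effects at the Arrow and calls WeaponTrace, an empty event here.
; Reload waits, refills ammo, then shows an animated reload bar widget.
; Sphere overlap adds a weapon component to an unarmed character and destroys the actor.
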(event `WeaponTrace`)

(event `WeaponFire`
  (`/Game/Blueprint/Libraries/BPML_Comparasions.Int <= Int` (`self.Ammo`)
    (:`True`
      (`self.Reload Weapon`))
    (:`False`
      (`/Engine/EditorBlueprintResources/StandardMacros.DecrementInt` (`self.Ammo`)
        (:`  `
          (`self.WeaponFireEffects`)
          (`self.WeaponTrace`))))))

(event `self.ReceiveBeginPlay`
  (set `self.Ammo` (`self.MaxAmmo`)))

(event `Reload Weapon`
  (`KismetSystemLibrary.Delay` (`self.Reloadtime`))
  (set `self.Ammo` (`self.MaxAmmo`))
  (bind _returnvalue (`|CreateWidget` "/Game/Blueprint/Weapons/WB_ReloadBar.WB_ReloadBar_C"))
  (`/Game/Blueprint/Weapons/WB_ReloadBar.ReloadAmmoAnimation` _returnvalue (`self.Reloadtime`))
  (`UserWidget.AddToViewport` _returnvalue 0))

(event `self.Sphere.OnComponentBeginOverlap`
  (params (OverlappedComponent :type "PrimitiveComponent Object Reference") (OtherActor :type "Actor Object Reference") (OtherComp :type "PrimitiveComponent Object Reference") (OtherBodyIndex :type Integer) (bFromSweep :type Boolean) (SweepResult :type "HitResult Structure (by ref)"))
  (bind _asbp_first_person_character (cast `/Game/FirstPerson/Blueprints/BP_FirstPersonCharacter` OtherActor))
  (`/Engine/EditorBlueprintResources/StandardMacros.IsValid` (`/Game/FirstPerson/Blueprints/BP_FirstPersonCharacter.Weapon` _asbp_first_person_character)
    (:`Is Not Valid`
      (`AddComponent|NODE_AddBP_Weapon_Component-0` :`self` _asbp_first_person_character)
      (`self.K2_DestroyActor`))))

(fn `UserConstructionScript`)

(fn `WeaponFireEffects`
  (bind _returnvalue (`SceneComponent.K2_GetComponentLocation` (`self.Arrow`)))
  (`GameplayStatics.SpawnEmitterAtLocation` (`self.Emitter Template`) _returnvalue (struct) (`self.Scale`))
  (`GameplayStatics.SpawnSoundAtLocation` (`self.Sound`) _returnvalue (struct) 1.0 1.0 0.0 null null))